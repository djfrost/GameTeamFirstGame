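; MainCharacter is a first-person character Blueprint with logic for interacting with objects and picking up items.
; Its interaction chain line-traces a short distance forward from the camera for one custom object type, then calls HasInteracted on an Interactableobject or, failing that cast, PickupItem on a BasicItem.
; That chain and two ChangeInteractionMode on/off calls have no triggering event, so none run, and the construction script is empty.
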(event Input|KeyboardEvents|LeftShift
  (params (Key :type Key%20Structure :default "AnyKey")))

(event Input|KeyboardEvents|Q
  (params (Key :type Key%20Structure :default "AnyKey")))

(fn ConstructionScript)